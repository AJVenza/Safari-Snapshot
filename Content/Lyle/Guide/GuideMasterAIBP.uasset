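; Guide NPC Blueprint that on BeginPlay walks to a target, roams or approaches the player, depending on AIState.
; Roam re-picks a random navigable point after each successful move; Follow moves to the player once and shows InteractText in a DialogueBP widget for five seconds.
; Follow also reads Dialogue table rows, but the NPCID filter into MyDialogue is unconnected.
; Interact increments LineCurrent and creates a dialogue widget that is never displayed.
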(event Custom|WalkTo
  ;[1 1 1] Walk from point A to point B
  (AI|AIMoveTo self "0, 0, 0" (Variables|Default|GetTarget_1) 5.0 false))

(event Custom|Roam
  ;[1 1 1] Roam around area
  (AI|AIMoveTo self (.RandomLocation (Class|NavigationSystemV1|GetRandomPointinNavigableRadius (Transformation|GetActorLocation) 5e+02 0 0)) 0 5.0 false
    (:OnSuccess
      (Utilities|FlowControl|Delay 2.0)
      (CallFunction|Roam))))

(event Custom|FindPlayer
  (AI|AIMoveTo self "0, 0, 0" (Game|GetPlayerCharacter 0) 5.0 false
    (:OnSuccess
      (bind _returnvalue (UserInterface|CreateWidget "/Game/Lyle/Guide/DialogueBP.DialogueBP_C" (Game|GetPlayerController 0)))
      (bind _output_get (Variables|Default|SetDialogueWindow _returnvalue))
      (UserInterface|Viewport|AddtoViewport _output_get 0)
      (Variables|/Game/Lyle/Guide/DialogueBP.DialogueBP_C|SetDialogueText (Variables|Default|GetDialogueWindow) (Variables|Default|GetInteractText))
      (Utilities|FlowControl|Delay 5.0)
      (Widget|RemovefromParent (Variables|Default|GetDialogueWindow))
      (Variables|Default|SetDialogueWindow 0))))

(event EventBeginPlay
  (switch Utilities|FlowControl|Switch|SwitchonGuideEnum (Variables|Default|GetAI_State)
    (:NewEnumerator0
      (CallFunction|Walkto))
    (:NewEnumerator1
      (CallFunction|Roam))
    (:NewEnumerator2
      (CallFunction|FindPlayer)
      (bind _outrownames (DataTable|GetDataTableRowNames "/Game/Lyle/Guide/Dialogue.Dialogue"))
      (for _array_element _outrownames
        (bind _returnvalue (Utilities|GetDataTableRow "/Game/Lyle/Guide/Dialogue.Dialogue" _array_element))))))

(event Collision|EventActorBeginOverlap
  (params (OtherActor :type Actor%20Object%20Reference)))

(event EventTick
  (params (DeltaSeconds :type Float%20%28single-precision%29)))

(event EventInteract
  (Math|Integer|IncrementInt (Variables|Default|GetLineCurrent)
    (:%20%20
      (CallFunction|DialogueCreate))))

(fn ConstructionScript)

(fn DialogueCreate
  (UserInterface|CreateWidget "/Game/Lyle/Guide/DialogueBP.DialogueBP_C" (Game|GetPlayerController 0)))