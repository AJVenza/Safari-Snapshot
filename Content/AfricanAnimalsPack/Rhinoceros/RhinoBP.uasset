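; Rhinoceros animal Blueprint with simple self-driven AI that roams, rests when tired and flees on sensed stimuli.
; Self-rescheduling one-second timers update Energy and Hunger, setting flags that DecideNextAction reads to choose behavior.
; Movement uses AI MoveTo to random reachable points, while rest and graze animations temporarily override the Animation Blueprint.
; Eat checks the ground's physical surface by downward trace, but nothing here calls it, and hunger halts new actions except fleeing.
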(event OnTargetPerceptionUpdated(AIPerception)
  (params (Actor :type Actor%20Object%20Reference) (Stimulus :type AI%20Stimulus%20Structure))
  ;[1 1 1] Detect noise
  (if (not (Variables|Default|GetShould%20Run?))
    (Variables|Default|SetShould%20Run? (.bSuccessfullySensed (Utilities|Struct|BreakAIStimulus Stimulus)))
    (CallFunction|DecideNextAction true)))

(event Custom|Decide%20Next%20Action
  (params (Skip%20Delay? :type Boolean))
  ;[1 1 1] Decide next action
  (if Skip%20Delay?
    _
    (else
      (Utilities|FlowControl|Delay (Math|Conversions|ToFloat(Integer) (Math|Random|RandomIntegerinRange 1 5)))))
  (if (Variables|Default|GetShould%20Run?)
    (CallFunction|RunAway)
    (elif (not (Variables|Default|GetIs%20Hungry?))
      (if (Variables|Default|GetIs%20Tired?)
        (CallFunction|Rest)
        (CallFunction|RegainEnergy)
        (else
          (CallFunction|RandomRoam))))))

(event Custom|Random%20Roam
  ;[1 1 1] Random roam
  (Variables|/Script/Engine.CharacterMovementComponent|SetMaxWalkSpeed (Variables|Character|GetCharacterMovement) 1.5e+02)
  (AI|AIMoveTo self (.RandomLocation (AI|Navigation|GetRandomReachablePointinRadius (Transformation|GetActorLocation) 1.5e+03 0 0)) 0 5.0 false
    (:OnSuccess
      (CallFunction|DecideNextAction false))))

(event Custom|Run%20Away
  ;[1 1 1] Run away
  (Variables|/Script/Engine.CharacterMovementComponent|SetMaxWalkSpeed (Variables|Character|GetCharacterMovement) 6e+02)
  (AI|AIMoveTo self (.RandomLocation (AI|Navigation|GetRandomReachablePointinRadius (Transformation|GetActorLocation) (Math|Random|RandomFloatinRange 2e+04 3e+04) 0 0)) 0 5.0 false
    (:OnSuccess
      (Variables|Default|SetShould%20Run? false)
      (CallFunction|DecideNextAction true))))

(event Custom|Rest
  ;[1 1 1] Sleeping anim
  (Components|Movement|StopMovementImmediately (Variables|Character|GetCharacterMovement))
  (CallFunction|PlayAnimation "/Game/AfricanAnimalsPack/Rhinoceros/Animations/ANIM_Rhinoceros_Death.ANIM_Rhinoceros_Death" false)
  (Utilities|FlowControl|Delay 1.4)
  (CallFunction|PlayAnimation "/Game/AfricanAnimalsPack/Rhinoceros/Animations/ANIM_Rhinoceros_Death.ANIM_Rhinoceros_Death" false)
  (Utilities|FlowControl|Delay (Math|Conversions|ToFloat(Integer) (Math|Random|RandomIntegerinRange 50 120)))
  (CallFunction|PlayAnimation "/Game/AfricanAnimalsPack/Rhinoceros/Animations/ANIM_Rhinoceros_GetHit.ANIM_Rhinoceros_GetHit" false)
  (Utilities|FlowControl|Delay 1.4)
  (CallFunction|StopAnimation)
  (Variables|Default|SetIs%20Tired? false)
  (CallFunction|DecideNextAction false)
  (CallFunction|DrainEnergy))

(event Custom|Drain%20Energy
  ;[1 1 1] Drain energy - normal = 125 seconds
  (if (not (Variables|Default|GetIs%20Tired?))
    (bind _output_get (Variables|Energy|SetEnergy (Math|Integer|Clamp(Integer) (- (Variables|Energy|GetEnergy) (Variables|Energy|GetEnergy%20Drain)) 0 (Variables|Energy|GetMax%20Energy))))
    (if (== _output_get 0)
      (Variables|Default|SetIs%20Tired? true)
      (CallFunction|DecideNextAction false)
      (else
        (Utilities|FlowControl|Delay 1.0)
        (CallFunction|DrainEnergy)))))

(event Custom|Regain%20Energy
  ;[1 1 1] Regain energy - takes 50 seconds
  (if (Variables|Default|GetIs%20Tired?)
    (bind _output_get (Variables|Energy|SetEnergy (Math|Integer|Clamp(Integer) (+ (Variables|Energy|GetEnergy) (Variables|Energy|GetEnergy%20Gain)) 0 (Variables|Energy|GetMax%20Energy))))
    (if (not (== _output_get (Variables|Energy|GetMax%20Energy)))
      (Utilities|FlowControl|Delay 1.0)
      (CallFunction|RegainEnergy))))

(event Custom|Eat
  ;[1 1 1] Est animation
  (bind _can_eat_ (Utilities|CanEat)
    (:Out
      (if _can_eat_
        (Components|Movement|StopMovementImmediately (Variables|Character|GetCharacterMovement))
        (CallFunction|AddHunger)
        (CallFunction|PlayAnimation "/Game/AfricanAnimalsPack/Rhinoceros/Animations/ANIM_Rhinoceros_WalkGraze.ANIM_Rhinoceros_WalkGraze" false)
        (Utilities|FlowControl|Delay 1.0)
        (CallFunction|PlayAnimation "/Game/AfricanAnimalsPack/Rhinoceros/Animations/ANIM_Rhinoceros_IdleGraze.ANIM_Rhinoceros_IdleGraze" true)
        (Utilities|FlowControl|Delay (Math|Conversions|ToFloat(Integer) (Math|Random|RandomIntegerinRange 3 10)))
        (CallFunction|PlayAnimation "/Game/AfricanAnimalsPack/Rhinoceros/Animations/ANIM_Rhino_Graze_End.ANIM_Rhino_Graze_End" false)
        (Utilities|FlowControl|Delay 1.0)
        (CallFunction|StopAnimation)
        (Variables|Default|SetIs%20Hungry? false)
        (CallFunction|DrainHunger)
        (CallFunction|DecideNextAction false)
        (else
          (CallFunction|DecideNextAction false)
          (Variables|Default|SetIs%20Hungry? false)
          (Utilities|FlowControl|Delay 5.0)
          (Variables|Default|SetIs%20Hungry? true))))))

(event Custom|Add%20Hunger
  ;[1 1 1] Regain hunger
  (if (Variables|Default|GetIs%20Hungry?)
    (bind _output_get (Variables|Hunger|SetHunger (Math|Integer|Clamp(Integer) (+ (Variables|Hunger|GetHunger) (Variables|Hunger|GetHunger%20Gain)) 0 (Variables|Hunger|GetMax%20Hunger))))
    (if (not (== _output_get (Variables|Hunger|GetMax%20Hunger)))
      (Utilities|FlowControl|Delay 1.0)
      (CallFunction|AddHunger))))

(event Custom|Drain%20Hunger
  ;[1 1 1] Drain hunger
  (if (not (Variables|Default|GetIs%20Hungry?))
    (bind _output_get (Variables|Hunger|SetHunger (Math|Integer|Clamp(Integer) (- (Variables|Hunger|GetHunger) (Variables|Hunger|GetHunger%20Drain)) 0 (Variables|Hunger|GetMax%20Hunger))))
    (if (== _output_get 0)
      (Variables|Default|SetIs%20Hungry? true)
      (CallFunction|DecideNextAction false)
      (else
        (Utilities|FlowControl|Delay 1.0)
        (CallFunction|DrainHunger)))))

(event EventBeginPlay
  ;[1 1 1] Set up blueprint
  (CallFunction|DecideNextAction false)
  (CallFunction|DrainEnergy)
  (CallFunction|DrainHunger))

(fn ConstructionScript)

(fn PlayAnimation
  (params (Animation :type Animation%20Asset%20Object%20Reference) (Should%20Loop? :type Boolean))
  (Components|Animation|PlayAnimation (Variables|Character|GetMesh) Animation Should%20Loop?))

(fn StopAnimation
  (Components|Animation|SetAnimationMode (Variables|Character|GetMesh) "AnimationBlueprint"))